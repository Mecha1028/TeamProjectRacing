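; Racing game mode that holds a shared SpeedOfBlocks value, set to a default on BeginPlay.
; SpeedGoesUp lowers the value and SpeedGoesDown raises it by a fixed step, clamped to a range, so a smaller number means faster.
; Lap-count checks that would show Win or Lose widgets, pause the game and show the cursor are disconnected and never run, and Tick is empty.
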(event Custom|SpeedGoesUp
  (Variables|Default|SetSpeedOfBlocks (Math|Float|Clamp(Float) (- (Variables|Default|GetSpeedOfBlocks) 5.0) 1.0 1e+01)))

(event Custom|SpeedGoesDown
  (Variables|Default|SetSpeedOfBlocks (Math|Float|Clamp(Float) (+ (Variables|Default|GetSpeedOfBlocks) 5.0) 1.0 1e+01)))

(event EventBeginPlay
  (Variables|Default|SetSpeedOfBlocks 6.0))

(event EventTick
  (params (DeltaSeconds :type Float%20%28single-precision%29)))

(fn ConstructionScript)