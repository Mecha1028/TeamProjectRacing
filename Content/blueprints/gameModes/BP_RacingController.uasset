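; Racing controller that turns gamepad, mouse and keyboard input into throttle, lane hops and drifting for the BP_CarChar it finds at BeginPlay.
; Tick passes accelerate, coast or brake state to the car's CarSpeed along the current spline.
; Lane input steps a clamped track index and sends a hop message to the car.
; Drifting on corners targets a signed max angle, lerped into CarControl each Tick; older drift logic remains disconnected.
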(event Custom|corner%20turn%20left
  ;[0.15 0.15 0.15 0.5] old drifting system
  ;;[0.15 0.15 0.15 0.5] drifting turning script
)

(event Custom|corner%20turn%20right
  ;[0.15 0.15 0.15 0.5] old drifting system
  ;;[0.15 0.15 0.15 0.5] drifting turning script
)

(event Custom|Reset%20Angle
  ;[0.15 0.15 0.15 0.5] sets target angle
  (Variables|Default|SetTargetAngle 0.0))

(event Custom|Accelerate
  (if (Variables|/Game/blueprints/BP_CarChar.BP_CarChar_C|GetHasControl (Variables|Default|GetCarREF))
    ;[0.15 0.15 0.15 0.5] speed changin nodes
    (if (not (Variables|Default|GetFreeWheel?))
      (if (Variables|Default|GetAccelClick)
        (Variables|Default|SetIsItAc true)
        (Default|CarSpeed (Variables|Default|GetCarREF) (Variables|Default|GetCar%20Max%20Speed) (Variables|Default|GetCar%20Acceleration) (Variables|Default|GetCar%20Deceleration) (Variables|Default|Getcurrent_Spline) (Variables|Default|GetIsItAc) :!label _label))
      (else
        (Variables|Default|SetCar%20Deceleration 0.05)
        (Variables|Default|SetIsItAc false)
        (goto _label)))))

(event Custom|Decelerate
  ;[0.15 0.15 0.15 0.5] speed changin nodes
  (if (Variables|/Game/blueprints/BP_CarChar.BP_CarChar_C|GetHasControl (Variables|Default|GetCarREF))
    (if (Variables|Default|GetDecelClick)
      (Variables|Default|SetCar%20Deceleration 0.1)
      (Variables|Default|SetIsItAc false)
      (Default|CarSpeed (Variables|Default|GetCarREF) (Variables|Default|GetCar%20Max%20Speed) (Variables|Default|GetCar%20Acceleration) (Variables|Default|GetCar%20Deceleration) (Variables|Default|Getcurrent_Spline) (Variables|Default|GetIsItAc)))))

(event Custom|set%20new%20spline
  (Class|BPILaneHop|OnHop(Message) (Variables|Default|GetCarREF) (Variables|Default|GetControllability%20Lane%20Hop) (Variables|Default|GettrackIndex)))

(event Custom|ChangeTargetOnCorner
  ;[0.15 0.15 0.15 0.5] sets target angle
  (if (Variables|/Game/blueprints/BP_CarChar.BP_CarChar_C|GetHasControl (Variables|Default|GetCarREF))
    (if (Variables|Default|GetIsItCW)
      (Variables|Default|SetTargetAngle (Variables|Default|GetmaxAngle))
      (else
        (Variables|Default|SetTargetAngle (* (Variables|Default|GetmaxAngle) -1.0))))))

(event EventTick
  (params (DeltaSeconds :type Float%20%28single-precision%29))
  (CallFunction|Accelerate)
  (CallFunction|Decelerate)
  (Variables|Default|SetCurrentAngle (Math|Float|Lerp (Variables|Default|GetCurrentAngle) (Variables|Default|GetTargetAngle) (Variables|Default|GetControllability)))
  (Default|CarControl (Variables|Default|GetCarREF) (Variables|Default|GetCurrentAngle)))

(event EventBeginPlay
  (bind _returnvalue (Actor|GetActorOfClass "/Game/blueprints/BP_CarChar.BP_CarChar_C"))
  (Variables|Default|SetCarREF _returnvalue)
  (Variables|Default|SetMax%20Track%20Index (- (Variables|Default|GetNumber%20of%20tracks) 1)))

(event Input|MouseEvents|LeftMouseButton
  (params (Key :type Key%20Structure :default "None"))
  (:Pressed
    (Variables|Default|SetFreeWheel? false)
    (Variables|Default|SetAccelClick true))
  (:Released
    (Variables|Default|SetFreeWheel? true)
    (Variables|Default|SetAccelClick false)))

(event Input|MouseEvents|RightMouseButton
  (params (Key :type Key%20Structure :default "None"))
  (:Pressed
    (Variables|Default|SetFreeWheel? false)
    (Variables|Default|SetDecelClick true))
  (:Released
    (Variables|Default|SetFreeWheel? true)
    (Variables|Default|SetDecelClick false)))

(event Input|KeyboardEvents|F
  (params (Key :type Key%20Structure :default "None"))
  ;[0.15 0.15 0.15 0.5] debug testing keys
)

(event Input|KeyboardEvents|Q
  (params (Key :type Key%20Structure :default "None"))
  ;[0.15 0.15 0.15 0.5] debug testing keys
)

(event Input|KeyboardEvents|A
  (params (Key :type Key%20Structure :default "None"))
  (:Pressed
    (if (Variables|/Game/blueprints/BP_CarChar.BP_CarChar_C|GetHasControl (Variables|Default|GetCarREF))
      ;[0.15 0.15 0.15 0.5] A and D control what index the lane uses and will then set the lane to be used
      (bind _result (Math|Integer|DecrementInt (Variables|Default|GettrackIndex))
        (:%20%20
          (Variables|Default|SettrackIndex (Math|Integer|Clamp(Integer) _result 0 (Variables|Default|GetMax%20Track%20Index)))
          (CallFunction|SetNewSpline))))))

(event Input|KeyboardEvents|D
  (params (Key :type Key%20Structure :default "None"))
  (:Pressed
    (if (Variables|/Game/blueprints/BP_CarChar.BP_CarChar_C|GetHasControl (Variables|Default|GetCarREF))
      ;[0.15 0.15 0.15 0.5] A and D control what index the lane uses and will then set the lane to be used
      (bind _result (Math|Integer|IncrementInt (Variables|Default|GettrackIndex))
        (:%20%20
          (Variables|Default|SettrackIndex (Math|Integer|Clamp(Integer) _result 0 (Variables|Default|GetMax%20Track%20Index)))
          (CallFunction|SetNewSpline))))))

(event Input|KeyboardEvents|SpaceBar
  (params (Key :type Key%20Structure :default "None"))
  ;[0.15 0.15 0.15 0.5] drifting controller#
  (:Pressed
    (Variables|Default|Setdrifting true)
    (if (Variables|Default|GetOnCorner)
      (CallFunction|ChangeTargetonCorner)
      (else
        (CallFunction|ResetAngle :!label _label))))
  (:Released
    (Variables|Default|Setdrifting false)
    (goto _label)))

(event Input|GamepadEvents|GamepadRightShoulder
  (params (Key :type Key%20Structure :default "None"))
  (:Pressed
    (Variables|Default|SetFreeWheel? false)
    (Variables|Default|SetDecelClick true))
  (:Released
    (Variables|Default|SetFreeWheel? true)
    (Variables|Default|SetDecelClick false)))

(event Input|GamepadEvents|GamepadLeftShoulder
  (params (Key :type Key%20Structure :default "None"))
  (:Pressed
    (Variables|Default|SetFreeWheel? false)
    (Variables|Default|SetAccelClick true))
  (:Released
    (Variables|Default|SetFreeWheel? true)
    (Variables|Default|SetAccelClick false)))

(event Input|GamepadEvents|GamepadDPadUp
  (params (Key :type Key%20Structure :default "None"))
  ;[0.15 0.15 0.15 0.5] drifting controller#
  (:Pressed
    (Variables|Default|Setdrifting true)
    (if (Variables|Default|GetOnCorner)
      (CallFunction|ChangeTargetonCorner)
      (else
        (CallFunction|ResetAngle :!label _label))))
  (:Released
    (Variables|Default|Setdrifting false)
    (goto _label)))

(event Input|GamepadEvents|GamepadDPadLeft
  (params (Key :type Key%20Structure :default "None"))
  (:Pressed
    (if (Variables|/Game/blueprints/BP_CarChar.BP_CarChar_C|GetHasControl (Variables|Default|GetCarREF))
      ;[0.15 0.15 0.15 0.5] A and D control what index the lane uses and will then set the lane to be used
      (bind _result (Math|Integer|DecrementInt (Variables|Default|GettrackIndex))
        (:%20%20
          (Variables|Default|SettrackIndex (Math|Integer|Clamp(Integer) _result 0 (Variables|Default|GetMax%20Track%20Index)))
          (CallFunction|SetNewSpline))))))

(event Input|GamepadEvents|GamepadDPadRight
  (params (Key :type Key%20Structure :default "None"))
  (:Pressed
    (if (Variables|/Game/blueprints/BP_CarChar.BP_CarChar_C|GetHasControl (Variables|Default|GetCarREF))
      ;[0.15 0.15 0.15 0.5] A and D control what index the lane uses and will then set the lane to be used
      (bind _result (Math|Integer|IncrementInt (Variables|Default|GettrackIndex))
        (:%20%20
          (Variables|Default|SettrackIndex (Math|Integer|Clamp(Integer) _result 0 (Variables|Default|GetMax%20Track%20Index)))
          (CallFunction|SetNewSpline))))))

(fn ConstructionScript)