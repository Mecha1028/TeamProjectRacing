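; BP_MoveActor is a car-like actor that travels along a referenced spline, starting on BeginPlay, with its mesh set at construction.
; A movement timeline maps progress to spline distance, updating world location and rotation.
; CarControl plays a drift timeline at a given controllability rate, blending a CarAngle yaw offset into that rotation.
; Speed-up and slow-down events adjust CarSpeed, then call ChangeSpeed to set play rate and play movement.
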(event Custom|Move%20Object
  (bind _splineref (Variables|Default|GetSplineRef))
  (bind _spline (Variables|/Game/blueprints/BP_SplineActor.BP_SplineActor_C|GetSpline _splineref))
  (Components|Timeline|SetPlayRate (Variables|Default|GetTarget_0) (/ 1.0 0.0))
  (bind _newtrack_0 (Timeline|movetimeLine Play)
    (:Update
      (Transformation|SetActorLocationAndRotation (Spline|GetLocationatDistanceAlongSpline _spline (Math|Float|Lerp 0.0 (Spline|GetSplineLength _spline) _newtrack_0) "World") (Math|Rotator|MakeRotator (.roll (Spline|GetRotationatDistanceAlongSpline _spline (Math|Float|Lerp 0.0 (Spline|GetSplineLength _spline) _newtrack_0) "World")) (.pitch (Spline|GetRotationatDistanceAlongSpline _spline (Math|Float|Lerp 0.0 (Spline|GetSplineLength _spline) _newtrack_0) "World")) (+ (* (stale EventCarControl car%20angle) (Math|Float|Lerp 0.0 1.0 (stale EventCarControl _turnval))) (.yaw (Spline|GetRotationatDistanceAlongSpline _spline (Math|Float|Lerp 0.0 (Spline|GetSplineLength _spline) _newtrack_0) "World"))))))))

(event Custom|change%20speed
  (bind _splineref (Variables|Default|GetSplineRef))
  (bind _spline (Variables|/Game/blueprints/BP_SplineActor.BP_SplineActor_C|GetSpline _splineref))
  (Components|Timeline|SetPlayRate (Variables|Default|GetTarget_0) (/ 1.0 0.0))
  (bind _newtrack_0 (Timeline|movetimeLine Play)
    (:Update
      (Transformation|SetActorLocationAndRotation (Spline|GetLocationatDistanceAlongSpline _spline (Math|Float|Lerp 0.0 (Spline|GetSplineLength _spline) _newtrack_0) "World") (Math|Rotator|MakeRotator (.roll (Spline|GetRotationatDistanceAlongSpline _spline (Math|Float|Lerp 0.0 (Spline|GetSplineLength _spline) _newtrack_0) "World")) (.pitch (Spline|GetRotationatDistanceAlongSpline _spline (Math|Float|Lerp 0.0 (Spline|GetSplineLength _spline) _newtrack_0) "World")) (+ (* (stale EventCarControl car%20angle) (Math|Float|Lerp 0.0 1.0 (stale EventCarControl _turnval))) (.yaw (Spline|GetRotationatDistanceAlongSpline _spline (Math|Float|Lerp 0.0 (Spline|GetSplineLength _spline) _newtrack_0) "World"))))))))

(event Custom|speed%20up
  (bind _output_get (Variables|Default|SetCarSpeed (+ (stale _output_get) (Variables|Default|GetaccelerationVal))))
  (CallFunction|ChangeSpeed))

(event Custom|slow%20down
  (bind _output_get (Variables|Default|SetCarSpeed (- (stale _output_get) (Variables|Default|GetdecelerationVal))))
  (CallFunction|ChangeSpeed))

(event EventBeginPlay
  (CallFunction|MoveObject))

(event EventCarControl
  (params (car%20angle :type Float%20%28double-precision%29) (controllability :type Float%20%28double-precision%29))
  (bind _splineref (Variables|Default|GetSplineRef))
  (bind _spline (Variables|/Game/blueprints/BP_SplineActor.BP_SplineActor_C|GetSpline _splineref))
  (Components|Timeline|SetPlayRate (Variables|Default|GetTarget_0) controllability)
  (bind _turnval (Timeline|DriftTimeLine Play)
    (:Update
      (Transformation|SetActorLocationAndRotation (Spline|GetLocationatDistanceAlongSpline _spline (Math|Float|Lerp 0.0 (Spline|GetSplineLength _spline) (stale Custom|Move%20Object _newtrack_0)) "World") (Math|Rotator|MakeRotator (.roll (Spline|GetRotationatDistanceAlongSpline _spline (Math|Float|Lerp 0.0 (Spline|GetSplineLength _spline) (stale Custom|Move%20Object _newtrack_0)) "World")) (.pitch (Spline|GetRotationatDistanceAlongSpline _spline (Math|Float|Lerp 0.0 (Spline|GetSplineLength _spline) (stale Custom|Move%20Object _newtrack_0)) "World")) (+ (* car%20angle (Math|Float|Lerp 0.0 1.0 _turnval)) (.yaw (Spline|GetRotationatDistanceAlongSpline _spline (Math|Float|Lerp 0.0 (Spline|GetSplineLength _spline) (stale Custom|Move%20Object _newtrack_0)) "World"))))))))

(fn ConstructionScript
  (Components|StaticMesh|SetStaticMesh (Variables|Default|GetCube) (Variables|Default|GetobjectMesh)))