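; Player car that rides spline tracks, with lane hopping, speed control, mesh-only yaw steering and fall-off handling.
; Lane hops and falls swap the spline and length-ratio speed correction; hops also update all obstacle boxes.
; Acceleration and deceleration feed ChangeSpeed, which sets timeline play rate.
; ChangeSpeed's hard-wired true branch plays only the fall-off timeline, which never moves the car, leaving the spline-following MoveTimeline branch unreachable.
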(event Custom|speed%20up
  ;[0.15 0.15 0.15 0.5] car speed code, alters speed variable and pings the movement script to change the speed
  (Development|PrintString "speed up")
  (Variables|Default|SetCarSpeed_0 (Math|Float|Clamp(Float) (+ (Variables|Default|GetCarSpeed_0) (stale EventCarSpeed acceleration)) 0.0 (Variables|Default|GetmaxCharSpeed)))
  (Development|PrintString (Utilities|String|ToString(Float) (stale Custom|slow%20down _output_get)))
  (CallFunction|ChangeSpeed))

(event Custom|change%20speed
  (bind _timetocomplete (Variables|Default|GettimeToComplete))
  (bind _carspeed_0 (Variables|Default|GetCarSpeed_0))
  (bind _splineref (Variables|Default|GetSplineRef))
  (bind _track_fix_num_char (Variables|Default|GetTrack%20Fix%20Num%20char))
  (bind _returnvalue (/ _carspeed_0 _track_fix_num_char))
  (bind _returnvalue_2 (* _timetocomplete 1e+02))
  (bind _returnvalue_3 (/ _returnvalue _returnvalue_2))
  ;[0.15 0.15 0.15 0.5] movement script, takes in pings from the laneswitch and the speed change functions.
  (if true
    (Components|Timeline|SetPlayRate (Variables|Default|GetFallOffTimeline) _returnvalue_3)
    (Timeline|FallOffTimeline Play
      (:Update
        (Default|GimmeThatSplie _splineref)))
    (else
      (Development|PrintString (Utilities|String|ToString(Float) _returnvalue))
      (Components|Timeline|SetPlayRate (Variables|Default|GetMoveTimeline) _returnvalue_3)
      (bind _speedtrack (Timeline|MoveTimeline Play)
        (:Update
          (bind _spline (Default|GimmeThatSplie _splineref))
          (Utilities|IsValid _spline
            (:Is%20Valid
              (Transformation|SetActorLocationAndRotation (Math|Vector|MakeVector (.x (Spline|GetLocationatDistanceAlongSpline _spline (Math|Float|Lerp 0.0 (Spline|GetSplineLength _spline) _speedtrack) "World")) (+ (Variables|Default|Gettrack%20offset) (.y (Spline|GetLocationatDistanceAlongSpline _spline (Math|Float|Lerp 0.0 (Spline|GetSplineLength _spline) _speedtrack) "World"))) (.z (Spline|GetLocationatDistanceAlongSpline _spline (Math|Float|Lerp 0.0 (Spline|GetSplineLength _spline) _speedtrack) "World"))) (Spline|GetRotationatDistanceAlongSpline _spline (Math|Float|Lerp 0.0 (Spline|GetSplineLength _spline) _speedtrack) "World")))
            (:Is%20Not%20Valid
              (Development|PrintString "not valid" false false))))))))

(event Custom|slow%20down
  ;[0.15 0.15 0.15 0.5] car speed code, alters speed variable and pings the movement script to change the speed
  (Development|PrintString "slow down")
  (bind _output_get (Variables|Default|SetCarSpeed_0 (Math|Float|Clamp(Float) (- (Variables|Default|GetCarSpeed_0) (stale EventCarSpeed deceleration)) 0.0 (Variables|Default|GetmaxCharSpeed))))
  (Development|PrintString (Utilities|String|ToString(Float) _output_get))
  (CallFunction|ChangeSpeed))

(event EventBeginPlay
  ;[0.15 0.15 0.15 0.5] set starting speed and check spline REF. collect all obstacle box actors to be used when the player changes track
  (Development|PrintString (Utilities|GetDisplayName (Variables|Default|GetSplineRef)))
  (Variables|Default|SetCarSpeed_0 0.0)
  (bind _outactors (Actor|GetAllActorsOfClass "/Game/blueprints/BP_ObbyBox.BP_ObbyBox_C"))
  (Variables|Default|SetObbyboxes _outactors))

(event EventOnHop
  (params (ControllabilityLaneHop :type Float%20%28double-precision%29) (SplineIndex :type Integer))
  ;[0.15 0.15 0.15 0.5] lane switch moves the car position to line up with other track and sets the new spline reference as well as the number to fix the speed on the new track
  (Variables|Default|SetSplineRef (Utilities|Array|Get(acopy) (Variables|Default|GetSplineArray) SplineIndex))
  (Variables|Default|SetControllability%20Lane%20Hop ControllabilityLaneHop)
  (Variables|Default|SetTrack%20Fix%20Num%20char (/ (Spline|GetSplineLength (Variables|/Game/blueprints/BP_SplineActor.BP_SplineActor_C|GetSpline (Variables|Default|GetSplineRef))) (Spline|GetSplineLength (Variables|/Game/blueprints/BP_SplineActor.BP_SplineActor_C|GetSpline (Variables|Default|Getspline%201)))))
  (CallFunction|ChangeSpeed)
  (for _array_element (Variables|Default|GetObbyboxes)
    (Default|ChangeFallOffPlace _array_element)))

(event EventOnFallOff
  (params (FallSpline :type BP%20Spline%20Actor%20Object%20Reference) (FallRate :type Float%20%28double-precision%29) (TrackFixer :type Float%20%28double-precision%29))
  ;[0.15 0.15 0.15 0.5] falling off code that sets the spline and speed while triggering the
  (Variables|Default|SetSplineRef FallSpline)
  (Variables|Default|SetCarSpeed_0 FallRate)
  (Variables|Default|SetTrack%20Fix%20Num%20char TrackFixer)
  (Variables|Default|SetIsFallenOff true)
  (CallFunction|ChangeSpeed))

(event EventTick
  (params (DeltaSeconds :type Float%20%28single-precision%29))
  ;[0.15 0.15 0.15 0.5] movement script, takes in pings from the laneswitch and the speed change functions.
)

(event EventCarSpeed
  (params (MaxSpeed :type Float%20%28double-precision%29) (acceleration :type Float%20%28double-precision%29) (deceleration :type Float%20%28double-precision%29) (SplineREF :type BP%20Spline%20Actor%20Object%20Reference) (isAccelerating :type Boolean))
  ;[0.15 0.15 0.15 0.5] car speed code, alters speed variable and pings the movement script to change the speed
  (Variables|Default|SetIs%20AcceleratingChar isAccelerating)
  (Variables|Default|SetmaxCharSpeed (+ MaxSpeed (Variables|Default|GetBoostToAdd)))
  (if (Variables|Default|GetIs%20AcceleratingChar)
    (CallFunction|SpeedUp)
    (else
      (CallFunction|SlowDown))))

(event EventCarControl
  (params (car%20angle :type Float%20%28double-precision%29) (controllability :type Float%20%28double-precision%29))
  (bind _maxangle (Variables|Default|GetmaxAngle))
  (bind _centraliser (Variables|Default|GetCentraliser))
  (bind _relativerotation (Variables|/Script/Engine.SceneComponent|GetRelativeRotation _centraliser))
  ;[0.15 0.15 0.15 0.5] rotation script, clamp doesn't function correctly but it does rotate just the mesh
  (Variables|Default|SetCharAngle (Math|Float|Clamp(Float) car%20angle (* _maxangle -1.0) _maxangle))
  (Development|PrintString (Utilities|String|ToString(Float) (+ (.yaw _relativerotation) (Variables|Default|GetCharAngle))))
  (Transformation|SetRelativeRotation _centraliser (Math|Rotator|MakeRotator (.roll _relativerotation) (.pitch _relativerotation) (+ (.yaw _relativerotation) (Variables|Default|GetCharAngle))) false false))

(fn ConstructionScript
  (Components|StaticMesh|SetStaticMesh (Variables|Default|GetStaticMesh) (Variables|Default|GetNew%20Mesh)))