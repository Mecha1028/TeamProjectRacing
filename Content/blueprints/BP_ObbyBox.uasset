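; BP_ObbyBox is a track trigger box that throws the car off at corners.
; On overlap it flags OnCorner on BP_RacingController, then calls OnFallOff on the car if its angle is too low and speed too high.
; The fall spline toggles between two fallback splines at BeginPlay and on changeFallOffPlace.
; Leaving clears the corner flag and sets the car's ShouldReset; the non-corner speed check does nothing.
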(event OnComponentBeginOverlap(Box)
  (params (OverlappedComponent :type Primitive%20Component%20Object%20Reference) (OtherActor :type Actor%20Object%20Reference) (OtherComp :type Primitive%20Component%20Object%20Reference) (OtherBodyIndex :type Integer) (bFromSweep :type Boolean) (SweepResult :type Hit%20Result%20Structure%20%28by%20ref%29))
  (bind _asbp_car_char (Utilities|Casting|CastToBP_CarChar OtherActor))
  (Variables|Default|SetAs%20BP%20Car%20Char _asbp_car_char)
  (Variables|/Game/blueprints/gameModes/BP_RacingController.BP_RacingController_C|SetOnCorner (Variables|Default|GetControllerREF) true)
  (Variables|Default|SetCar%20Speed%200 (Variables|/Game/blueprints/BP_CarChar.BP_CarChar_C|GetCarSpeed_0 (Variables|Default|GetAs%20BP%20Car%20Char)))
  (Variables|Default|SetChar%20Angle (Variables|/Game/blueprints/BP_CarChar.BP_CarChar_C|GetCharAngle (Variables|Default|GetAs%20BP%20Car%20Char)))
  (if (Variables|Default|GetIsCorner)
    (if (and (< (Variables|Default|GetChar%20Angle) (Variables|Default|GetRequiredAngle)) (>= (Variables|Default|GetCar%20Speed%200) (Variables|Default|GetrequiredSpeed)))
      (Default|OnFallOff (Variables|Default|GetAs%20BP%20Car%20Char) (Variables|Default|GetnewSpline) (Variables|Default|GetfallSplineSpeed) 1.0))
    (elif (>= (Variables|Default|GetCar%20Speed%200) (Variables|Default|GetrequiredSpeed))
      _)))

(event OnComponentEndOverlap(Box)
  (params (OverlappedComponent :type Primitive%20Component%20Object%20Reference) (OtherActor :type Actor%20Object%20Reference) (OtherComp :type Primitive%20Component%20Object%20Reference) (OtherBodyIndex :type Integer))
  (Variables|/Game/blueprints/gameModes/BP_RacingController.BP_RacingController_C|SetOnCorner (Variables|Default|GetControllerREF) false)
  (Variables|/Game/blueprints/BP_CarChar.BP_CarChar_C|SetShouldReset (Variables|Default|GetAs%20BP%20Car%20Char) true))

(event Custom|changeFallOffPlace
  (if (Variables|Default|GetIsFirstTrack)
    (Variables|Default|SetnewSpline (Variables|Default|GetfallBackspline2))
    (Variables|Default|SetIsFirstTrack false)
    (else
      (Variables|Default|SetnewSpline (Variables|Default|GetfallBackspline1))
      (Variables|Default|SetIsFirstTrack true))))

(event EventBeginPlay
  (bind _returnvalue (Actor|GetActorOfClass "/Game/blueprints/gameModes/BP_RacingController.BP_RacingController_C"))
  (Variables|Default|SetControllerREF _returnvalue)
  (if (Variables|Default|GetIsFirstTrack)
    (Variables|Default|SetnewSpline (Variables|Default|GetfallBackspline2))
    (Variables|Default|SetIsFirstTrack false)
    (else
      (Variables|Default|SetnewSpline (Variables|Default|GetfallBackspline1))
      (Variables|Default|SetIsFirstTrack true))))

(fn ConstructionScript)