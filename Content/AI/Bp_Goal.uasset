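; Bp_Goal is a trigger volume that counts laps for AI spline cars in the racing game.
; When a carspline1 with Canscore set enters the Box, it increments the shared Ailaps counter on BP_RacingGameMode and prints the new total.
; It clears the car's Canscore on scoring and sets it again when the car's overlap ends, guarding against repeat counts within one crossing.
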(event OnComponentBeginOverlap(Box)
  (params (OverlappedComponent :type Primitive%20Component%20Object%20Reference) (OtherActor :type Actor%20Object%20Reference) (OtherComp :type Primitive%20Component%20Object%20Reference) (OtherBodyIndex :type Integer) (bFromSweep :type Boolean) (SweepResult :type Hit%20Result%20Structure%20%28by%20ref%29))
  (bind _ascarspline_1 (Utilities|Casting|CastTocarspline1 OtherActor))
  (if (Variables|/Game/AI/carspline1.carspline1_C|Getcanscore _ascarspline_1)
    (bind _asbp_racing_game_mode (Utilities|Casting|CastToBP_RacingGameMode (Game|GetGameMode)))
    (bind _output_get (Variables|/Game/blueprints/gameModes/BP_RacingGameMode.BP_RacingGameMode_C|Setailaps _asbp_racing_game_mode (+ (Variables|/Game/blueprints/gameModes/BP_RacingGameMode.BP_RacingGameMode_C|Getailaps _asbp_racing_game_mode) 1)))
    (Variables|/Game/AI/carspline1.carspline1_C|Setcanscore _ascarspline_1 false)
    (Development|PrintString (Utilities|String|ToString(Integer) _output_get))))

(event OnComponentEndOverlap(Box)
  (params (OverlappedComponent :type Primitive%20Component%20Object%20Reference) (OtherActor :type Actor%20Object%20Reference) (OtherComp :type Primitive%20Component%20Object%20Reference) (OtherBodyIndex :type Integer))
  (bind _ascarspline_1 (Utilities|Casting|CastTocarspline1 OtherActor))
  (Variables|/Game/AI/carspline1.carspline1_C|Setcanscore _ascarspline_1 true))

(event EventBeginPlay)

(event EventTick
  (params (DeltaSeconds :type Float%20%28single-precision%29)))

(fn ConstructionScript)