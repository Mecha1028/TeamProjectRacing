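; BP_goalplayer is a scoring trigger that awards points to BP_CarChar cars entering its R component.
; On begin overlap, a car whose Canscores flag is set gains one point, has the flag cleared and gets its new score printed.
; End overlap sets the flag again, so each car scores once until it leaves a trigger.
; Score and flag both live on the car, and the goal keeps no state.
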(event OnComponentBeginOverlap(r)
  (params (OverlappedComponent :type Primitive%20Component%20Object%20Reference) (OtherActor :type Actor%20Object%20Reference) (OtherComp :type Primitive%20Component%20Object%20Reference) (OtherBodyIndex :type Integer) (bFromSweep :type Boolean) (SweepResult :type Hit%20Result%20Structure%20%28by%20ref%29))
  (bind _asbp_car_char (Utilities|Casting|CastToBP_CarChar OtherActor))
  (if (Variables|/Game/blueprints/BP_CarChar.BP_CarChar_C|Getcanscores _asbp_car_char)
    (bind _output_get (Variables|/Game/blueprints/BP_CarChar.BP_CarChar_C|Setscore _asbp_car_char (+ (Variables|/Game/blueprints/BP_CarChar.BP_CarChar_C|Getscore _asbp_car_char) 1)))
    (Variables|/Game/blueprints/BP_CarChar.BP_CarChar_C|Setcanscores _asbp_car_char false)
    (Development|PrintString (Utilities|String|ToString(Integer) _output_get))))

(event OnComponentEndOverlap(r)
  (params (OverlappedComponent :type Primitive%20Component%20Object%20Reference) (OtherActor :type Actor%20Object%20Reference) (OtherComp :type Primitive%20Component%20Object%20Reference) (OtherBodyIndex :type Integer))
  (bind _asbp_car_char (Utilities|Casting|CastToBP_CarChar OtherActor))
  (Variables|/Game/blueprints/BP_CarChar.BP_CarChar_C|Setcanscores _asbp_car_char true))

(event EventBeginPlay)

(event Collision|EventActorBeginOverlap
  (params (OtherActor :type Actor%20Object%20Reference)))

(event EventTick
  (params (DeltaSeconds :type Float%20%28single-precision%29)))

(fn ConstructionScript)